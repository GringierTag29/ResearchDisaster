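; Player character Blueprint that handles basic movement, mouse-look style turning, jumping and hold-to-sprint.
; Axis inputs drive controller yaw and pitch and add movement along the actor's forward and right vectors.
; Sprint press and release set IsSprinting, then call UpdateMovementSpeed to switch max walk speed between normal and sprint values.
; That call targets player 0's character through a cast made only on press, which the release path reuses.
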(event `InputAxis|MoveForward`
  (params (AxisValue :type "Float (single-precision)"))
  ;[1 1 1] Jump move
  (`self.AddMovementInput` (`self.GetActorForwardVector`) AxisValue))

(event `InputAxis|LookUp`
  (params (AxisValue :type "Float (single-precision)"))
  ;[1 1 1] Turn
  (`self.AddControllerPitchInput` AxisValue))

(event `InputAxis|Turn`
  (params (AxisValue :type "Float (single-precision)"))
  ;[1 1 1] Turn
  (`self.AddControllerYawInput` AxisValue))

(event `InputAxis|MoveRight`
  (params (AxisValue :type "Float (single-precision)"))
  ;[1 1 1] Jump move
  (`self.AddMovementInput` (`self.GetActorRightVector`) AxisValue))

(event `InputAction|Jump`
  (params (Key :type "Key Structure"))
  ;[1 1 1] Jump move
  (:`Pressed`
    (`self.Jump`)))

(event `InputAction|Sprint` :consume false
  (params (Key :type "Key Structure"))
  ;[1 1 1] Sprint
  (:`Pressed`
    (set `self.IsSprinting` true)
    (bind _asbp_player_character (cast `/Game/Blueprints/Player/BP_PlayerCharacter` (`GameplayStatics.GetPlayerCharacter` 0)))
    (`self.UpdateMovementSpeed` _asbp_player_character :!label _label))
  (:`Released`
    (set `self.IsSprinting` false)
    (goto _label)))

(fn `UpdateMovementSpeed`
  (bind _charactermovement (`self.CharacterMovement`))
  (if (`self.IsSprinting`)
    (set `CharacterMovementComponent.MaxWalkSpeed` 7500.0 _charactermovement)
    (else
      (set `CharacterMovementComponent.MaxWalkSpeed` 500.0 _charactermovement))))

(fn `UserConstructionScript`)